(event Custom|CE_GenMesh
  (params (SM :type Static%20Mesh%20Component%20Object%20Reference))
  (bind _new_mesh (Variables|Default|GetNew%20Mesh))
  (Components|StaticMesh|SetStaticMesh SM (Utilities|Array|Get(acopy) _new_mesh (Math|Random|RandomInteger (Utilities|Array|Length _new_mesh)))))

(event Custom|CE_Create
  (params (Z%20Offset :type Float%20%28double-precision%29) (X%20Offset :type Float%20%28double-precision%29) (Y%20Offset :type Float%20%28double-precision%29) (Rot%20Offset :type Float%20%28double-precision%29))
  (bind _staticmesh (Variables|Default|GetStaticMesh))
  (bind _returnvalue (Transformation|GetRelativeTransform _staticmesh))
  (bind _returnvalue_2 (AddComponent|AddStaticMeshComponent false (Math|Transform|MakeTransform (Math|Vector|MakeVector (+ (.x (.location _returnvalue)) X%20Offset) (+ (.y (.location _returnvalue)) Y%20Offset) (+ (.z (.location _returnvalue)) Z%20Offset)) (Math|Rotator|MakeRotator (.roll (.rotation _returnvalue)) (.pitch (.rotation _returnvalue)) (+ Rot%20Offset (.yaw (.rotation _returnvalue)))) (.scale _returnvalue))))
  (CallFunction|CEGenMesh _returnvalue_2))

(event Custom|CE_Offsets
  (params (Scale :type Float%20%28double-precision%29) (X%20Offset :type Float%20%28double-precision%29) (Y%20Offset :type Float%20%28double-precision%29) (Z%20Offset :type Float%20%28double-precision%29) (Rot%20Offset :type Float%20%28double-precision%29) (X :type Float%20%28double-precision%29) (Y :type Float%20%28double-precision%29))
  (Variables|Default|SetScale Scale)
  (Variables|Default|SetRot%20Offset Rot%20Offset)
  (Variables|Default|SetX%20Offset X%20Offset)
  (Variables|Default|SetY%20Offset Y%20Offset)
  (Variables|Default|SetY Y)
  (Variables|Default|SetX X)
  (Variables|Default|SetZ%20Offset Z%20Offset))

(event Custom|CE_%20Build
  (params (Scale :type Float%20%28double-precision%29) (X%20Offset :type Float%20%28double-precision%29) (Y%20Offset :type Float%20%28double-precision%29) (Z%20Offset :type Float%20%28double-precision%29) (Rot%20Offset :type Float%20%28double-precision%29) (X :type Float%20%28double-precision%29) (Y :type Float%20%28double-precision%29))
  (CallFunction|CEOffsets Scale X%20Offset Y%20Offset Z%20Offset Rot%20Offset X Y)
  (if (> (Variables|Default|GetScale) 0.0) :!label _label
    (CallFunction|CECreate 0.0 0.0 0.0 0.0)
    (Variables|Default|SetScale (- (Variables|Default|GetScale) 1.0))
    (Utilities|FlowControl|Delay 0.0001)
    (goto _label)))

(event Custom|CE_Start
  (bind _empty (Variables|Default|GetEmpty))
  (bind _floors (Variables|Default|GetFloors))
  (if (not (== _floors 0))
    (Utilities|Array|SetArrayElem _empty (- _floors 1) 0.0 true)
    (for _array_element _empty
      (CallFunction|Floor (* (Math|Random|RandomFloat) 1e+01) 0.0 0.0 (Variables|Default|GetZ%20Offset) 0.0 0.0 0.0)
      (Variables|Default|SetZ%20Offset (+ (Variables|Default|GetZ%20Offset) 3.5e+02)))
    (Utilities|Array|Clear _empty)))

(event Custom|CE_Floor
  (params (Scale :type Float%20%28double-precision%29) (Z%20Offset :type Float%20%28double-precision%29))
  ;[0.15 0.15 0.15 0.5] Backup Floor
  (CallFunction|CEBuild 0.0 0.0 3e+02 0.0 0.0 0.0 3e+02)
  (Utilities|FlowControl|Delay 0.1)
  (CallFunction|CEBuild 1e+01 -3e+02 (- (Variables|Default|GetY%20Offset) 3e+02) (Variables|Default|GetZ%20Offset) 9e+01 -3e+02 0.0)
  (Utilities|FlowControl|Delay 0.1)
  (CallFunction|CEBuild 1e+01 (+ (Variables|Default|GetX%20Offset) 3e+02) (- (Variables|Default|GetY%20Offset) 3e+02) (Variables|Default|GetZ%20Offset) 1.8e+02 0.0 -3e+02)
  (Utilities|FlowControl|Delay 0.1)
  (CallFunction|CEBuild 1e+01 (+ (Variables|Default|GetX%20Offset) 3e+02) (- (Variables|Default|GetY%20Offset) -3e+02) (Variables|Default|GetZ%20Offset) 2.7e+02 3e+02 0.0))

(event Custom|CE_Tile
  (params (Z%20Offset :type Float%20%28double-precision%29) (X%20Offset :type Float%20%28double-precision%29) (Y%20Offset :type Float%20%28double-precision%29) (Rot%20Offset :type Float%20%28double-precision%29))
  (bind _staticmesh (Variables|Default|GetStaticMesh))
  (bind _returnvalue (Transformation|GetRelativeTransform _staticmesh))
  (bind _returnvalue_2 (AddComponent|AddStaticMeshComponent false (Math|Transform|MakeTransform (Math|Vector|MakeVector (+ (.x (.location _returnvalue)) Z%20Offset) (+ (.y (.location _returnvalue)) X%20Offset) (+ (.z (.location _returnvalue)) Y%20Offset)) (Math|Rotator|MakeRotator (.roll (.rotation _returnvalue)) 9e+01 (+ (.yaw (.rotation _returnvalue)) Rot%20Offset)) (.scale _returnvalue))))
  (CallFunction|CEGenMesh _returnvalue_2))

(event EventBeginPlay
  (CallFunction|CEStart))

(event EventTick
  (params (DeltaSeconds :type Float%20%28single-precision%29))
  ;[0.15 0.1362 0 0.5] TEST
)

(fn ConstructionScript
  (CallFunction|CEStart))

(fn Floor
  (params (Scale :type Float%20%28double-precision%29) (Offset%20X :type Float%20%28double-precision%29) (Offset%20Y :type Float%20%28double-precision%29) (Offset%20Z :type Float%20%28double-precision%29) (X :type Float%20%28double-precision%29) (Y :type Float%20%28double-precision%29) (Rot%20Offset%20 :type Float%20%28double-precision%29))
  (LocalVariables|SetScaleLoc Scale)
  (LocalVariables|SetOffset%20X%20Loc Offset%20X)
  (LocalVariables|SetOffset%20Y%20Loc Offset%20Y)
  (LocalVariables|SetOffset%20Z%20Loc Offset%20Z)
  (LocalVariables|SetX%20Loc X)
  (LocalVariables|SetY%20Loc Y)
  (LocalVariables|SetRot%20Offset%20Loc0 Rot%20Offset%20)
  (LocalVariables|SetScaleY (* (LocalVariables|GetScaleLoc) (Math|Float|Clamp(Float) (Math|Random|RandomFloat) 0.9)))
  (LocalVariables|SetScaleX (* (LocalVariables|GetScaleLoc) (Math|Float|Clamp(Float) (Math|Random|RandomFloat) 0.9)))
  (bind _y_out (CallFunction|Build (LocalVariables|GetScaleLoc) 0.0 3e+02 (LocalVariables|GetOffset%20Z%20Loc) 0.0 3e+02 0.0 (LocalVariables|GetScaleY)))
  (bind (_x_out _y_out_2) (CallFunction|Build (LocalVariables|GetScaleLoc) -3e+02 (- _y_out 3e+02) (LocalVariables|GetOffset%20Z%20Loc) -3e+02 0.0 9e+01 (LocalVariables|GetScaleX)))
  (bind (_x_out_2 _y_out_3) (CallFunction|Build (LocalVariables|GetScaleLoc) (+ _x_out 3e+02) (- _y_out_2 3e+02) (LocalVariables|GetOffset%20Z%20Loc) 0.0 -3e+02 1.8e+02 (LocalVariables|GetScaleY)))
  (bind (_x_out_3 _y_out_4) (CallFunction|Build (LocalVariables|GetScaleLoc) (+ _x_out_2 3e+02) (- _y_out_3 -3e+02) (LocalVariables|GetOffset%20Z%20Loc) 3e+02 0.0 2.7e+02 (LocalVariables|GetScaleX)))
  (return _x_out_3 _y_out_4))

(fn Build
  (params (Scale :type Float%20%28double-precision%29) (X%20Offset :type Float%20%28double-precision%29) (Y%20Offset :type Float%20%28double-precision%29) (Z%20Offset :type Float%20%28double-precision%29) (X :type Float%20%28double-precision%29) (Y :type Float%20%28double-precision%29) (Rot%20Offset :type Float%20%28double-precision%29) (CeilingTiles :type Float%20%28double-precision%29))
  (bind _empty2 (LocalVariables|GetEmpty2))
  (LocalVariables|SetX%20Offset%20Loc X%20Offset)
  (LocalVariables|SetY%20Offset%20Loc Y%20Offset)
  (LocalVariables|SetZ%20Offset%20Loc Z%20Offset)
  (LocalVariables|SetRot%20Offset%20Loc Rot%20Offset)
  (LocalVariables|SetX0 X)
  (LocalVariables|SetTiles CeilingTiles)
  (LocalVariables|SetY0 Y)
  (Utilities|Array|SetArrayElem _empty2 (Math|Float|Truncate Scale) 1.0 true)
  (for (_ _array_index) _empty2
    (CallFunction|CECreate (LocalVariables|GetZ%20Offset%20Loc) (LocalVariables|GetX%20Offset%20Loc) (LocalVariables|GetY%20Offset%20Loc) (LocalVariables|GetRot%20Offset%20Loc))
    (bind _output_get (LocalVariables|SetY%20Offset%20Loc (+ (LocalVariables|GetY%20Offset%20Loc) (LocalVariables|GetY0))))
    (bind _output_get_2 (LocalVariables|SetX%20Offset%20Loc (+ (LocalVariables|GetX%20Offset%20Loc) (LocalVariables|GetX0)))))
  (return _output_get_2 _output_get))

(fn Create)