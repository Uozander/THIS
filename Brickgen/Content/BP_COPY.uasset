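; BP_COPY is a self-replicating actor that lays out a square outline of BP_Generator spawns.
; Each instance spawns a generator above itself after a short delay, rotated 90 degrees when DirectionX is false.
; The Original instance loops with delays to spawn copies along two X rows, then BuildY fills the two Y sides.
; Spacing follows the actor's X scale, the Scale variable sets side length, and each copy's DirectionX marks its side.
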(event Custom|CE_GEN
  (params (Direction%20X :type Boolean))
  (bind _returnvalue (Transformation|GetActorTransform))
  (bind _returnvalue_2 (Transformation|GetActorTransform))
  (if Direction%20X
    (Game|SpawnActorfromClass "/Game/BP_Generator.BP_Generator_C" (Math|Transform|MakeTransform (Math|Vector|MakeVector (.x (.location _returnvalue_2)) (.y (.location _returnvalue_2)) (+ (.z (.location _returnvalue_2)) (* (.X (Math|Vector|BreakVector (.scale _returnvalue_2))) 5e+02)))) "Undefined" "MultiplyWithRoot" 0 0)
    (else
      (Game|SpawnActorfromClass "/Game/BP_Generator.BP_Generator_C" (Math|Transform|MakeTransform (Math|Vector|MakeVector (.x (.location _returnvalue)) (.y (.location _returnvalue)) (+ (.z (.location _returnvalue)) (* (.X (Math|Vector|BreakVector (.scale _returnvalue))) 5e+02))) "0.000000,90.000000,0.000000") "Undefined" "MultiplyWithRoot" 0 0))))

(event Custom|BuildY
  (bind _returnvalue (Transformation|GetActorTransform))
  (bind _x (Math|Vector|BreakVector (.scale _returnvalue)))
  (bind _returnvalue_2 (* _x 1e+03))
  (Variables|Default|SetBonusY (- (Variables|Default|GetBonusY) _returnvalue_2))
  (bind _returnvalue_3 (Game|SpawnActorfromClass "BP_COPY_C" (Math|Transform|MakeTransform (Math|Vector|MakeVector (+ (.x (.location _returnvalue)) (Variables|Default|GetBonusX)) (+ (.y (.location _returnvalue)) (Variables|Default|GetBonusY)) (.z (.location _returnvalue))) (.rotation _returnvalue) (.scale _returnvalue)) "Undefined" "MultiplyWithRoot" 0 0 :!label _label))
  (Variables|BP_COPY_C|SetDirection%20X _returnvalue_3 true)
  (if (>= (Variables|Default|GetBonusY) (* _x 9e+01))
    (Variables|Default|SetBonusY (- (Variables|Default|GetBonusY) _returnvalue_2))
    (Utilities|FlowControl|Delay 0.1)
    (goto _label)
    (elif (not (== (Variables|Default|GetBonusX) 0.0))
      (Variables|Default|SetBonusX 0.0)
      (Variables|Default|SetBonusY (+ (* (Variables|Default|GetScale) _returnvalue_2) (Variables|Default|GetBonusY)))
      (Utilities|FlowControl|Delay 0.1)
      (goto _label))))

(event EventBeginPlay
  (bind _returnvalue (Transformation|GetActorTransform))
  (bind _x (Math|Vector|BreakVector (.scale _returnvalue)))
  (bind _returnvalue_2 (* _x 1e+03))
  (Utilities|FlowControl|Delay 0.2)
  (CallFunction|CEGEN (Variables|Default|GetDirection%20X))
  (Variables|Default|SetBonusX _returnvalue_2)
  (if (Variables|Default|GetOriginal)
    (bind _returnvalue_3 (Game|SpawnActorfromClass "BP_COPY_C" (Math|Transform|MakeTransform (Math|Vector|MakeVector (+ (.x (.location _returnvalue)) (Variables|Default|GetBonusX)) (+ (.y (.location _returnvalue)) (Variables|Default|GetBonusY)) (.z (.location _returnvalue))) (.rotation _returnvalue) (.scale _returnvalue)) "Undefined" "MultiplyWithRoot" 0 0 :!label _label))
    (Variables|BP_COPY_C|SetDirection%20X _returnvalue_3 false)
    (if (>= (Variables|Default|GetScale) (/ (Variables|Default|GetBonusX) _returnvalue_2))
      (Variables|Default|SetBonusX (+ _returnvalue_2 (Variables|Default|GetBonusX)))
      (Utilities|FlowControl|Delay 0.1)
      (goto _label)
      (elif (>= (Variables|Default|GetBonusY) (* _returnvalue_2 (Variables|Default|GetScale)))
        (CallFunction|BuildY)
        (else
          (Variables|Default|SetBonusX 0.0)
          (Variables|Default|SetBonusY (+ (* (Variables|Default|GetScale) _returnvalue_2) (Variables|Default|GetBonusY)))
          (Utilities|FlowControl|Delay 0.1)
          (goto _label))))))

(fn ConstructionScript)