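; BP_Generator procedurally grows a randomized, tower-like structure from static mesh components at BeginPlay.
; Spawn_Tier recursively stacks random Bases meshes upward from Cube with short delays, using Scale as a shared countdown.
; Tiers occasionally branch through recursive Side_Tier offsets or get thin, randomly chosen Decals meshes on their sides via CE_Decal.
; BuildY, marked DEP, and its disconnected grid loop spawn further generators but are never triggered here.
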(event Custom|Spawn_Tier
  (params (SM :type Static%20Mesh%20Component%20Object%20Reference))
  (bind _returnvalue (Transformation|GetRelativeTransform SM))
  (bind _bases (Variables|Default|GetBases))
  (Utilities|FlowControl|Delay 0.01)
  (if (>= (Variables|Default|GetScale) 0.1)
    (Variables|Default|SetScale (- (Variables|Default|GetScale) 1.0))
    (bind _returnvalue_2 (AddComponent|AddStaticMeshComponent false (Math|Transform|MakeTransform (Math|Vector|MakeVector (.x (.location _returnvalue)) (.y (.location _returnvalue)) (+ (.z (.location _returnvalue)) (* (.Z (Math|Vector|BreakVector (.scale _returnvalue))) (Variables|Default|GetBase%20Offset)))) (.rotation _returnvalue) (* (Transformation|GetActorScale3D) (Variables|Default|GetSide%20Size)))))
    (Components|StaticMesh|SetStaticMesh _returnvalue_2 (Utilities|Array|Get(acopy) _bases (Math|Random|RandomInteger (Utilities|Array|Length _bases))))
    (CallFunction|SpawnTier _returnvalue_2)
    (if (>= (Math|Random|RandomFloat) 0.99)
      (CallFunction|SideTier _returnvalue_2)
      (if (>= (Math|Random|RandomFloat) 0.1)
        (CallFunction|SideTier _returnvalue_2))
      (elif (Math|Random|RandomBool)
        (CallFunction|CEDecal "NegX" _returnvalue_2)
        (CallFunction|CEDecal "PosX" _returnvalue_2)
        (CallFunction|CEDecal "PosY" _returnvalue_2)
        (CallFunction|CEDecal "NegY" _returnvalue_2)))))

(event Custom|Side_Tier
  (params (SM :type Static%20Mesh%20Component%20Object%20Reference))
  (bind _returnvalue (Transformation|GetRelativeTransform SM))
  (bind _returnvalue_2 (Transformation|GetRelativeTransform SM))
  (bind _returnvalue_3 (Transformation|GetRelativeTransform SM))
  (bind _returnvalue_4 (Transformation|GetRelativeTransform SM))
  (bind _offset (Variables|Default|GetOffset))
  (bind _offset_2 (Variables|Default|GetOffset))
  (bind _decals (Variables|Default|GetDecals))
  (bind _decals_2 (Variables|Default|GetDecals))
  (bind _decals_3 (Variables|Default|GetDecals))
  (bind _decals_4 (Variables|Default|GetDecals))
  (if (>= (Math|Random|RandomFloat) 0.1)
    (if (Math|Random|RandomBool)
      (if (Math|Random|RandomBool)
        (bind _returnvalue_5 (AddComponent|AddStaticMeshComponent false (Math|Transform|MakeTransform (Math|Vector|MakeVector (+ (.x (.location _returnvalue_4)) _offset) (.y (.location _returnvalue_4)) (.z (.location _returnvalue_4))) (.rotation _returnvalue_4) (* (.scale _returnvalue_4) (Variables|Default|GetSide%20Size)))))
        (Components|StaticMesh|SetStaticMesh _returnvalue_5 (Utilities|Array|Get(acopy) _decals_4 (Math|Random|RandomInteger (Utilities|Array|Length _decals_4))))
        (CallFunction|SpawnTier _returnvalue_5)
        (if (>= (Math|Random|RandomFloat) 0.1)
          (CallFunction|SideTier _returnvalue_5)
          (CallFunction|CEDecal "NegX" _returnvalue_5))
        (else
          (bind _returnvalue_6 (AddComponent|AddStaticMeshComponent false (Math|Transform|MakeTransform (Math|Vector|MakeVector (+ (.x (.location _returnvalue_3)) _offset) (.y (.location _returnvalue_3)) (.z (.location _returnvalue_3))) (.rotation _returnvalue_3) (* (.scale _returnvalue_3) (Variables|Default|GetSide%20Size)))))
          (Components|StaticMesh|SetStaticMesh _returnvalue_6 (Utilities|Array|Get(acopy) _decals_3 (Math|Random|RandomInteger (Utilities|Array|Length _decals_3))))
          (CallFunction|SpawnTier _returnvalue_6)
          (if (>= (Math|Random|RandomFloat) 0.1)
            (CallFunction|SideTier _returnvalue_6)
            (CallFunction|CEDecal "PosX" _returnvalue_6))))
      (elif (Math|Random|RandomBool)
        (bind _returnvalue_7 (AddComponent|AddStaticMeshComponent false (Math|Transform|MakeTransform (Math|Vector|MakeVector (.x (.location _returnvalue)) (+ (.y (.location _returnvalue)) _offset_2) (.z (.location _returnvalue))) (.rotation _returnvalue) (* (.scale _returnvalue) (Variables|Default|GetSide%20Size)))))
        (Components|StaticMesh|SetStaticMesh _returnvalue_7 (Utilities|Array|Get(acopy) _decals_2 (Math|Random|RandomInteger (Utilities|Array|Length _decals_2))))
        (CallFunction|SpawnTier _returnvalue_7)
        (if (>= (Math|Random|RandomFloat) 0.1)
          (CallFunction|SideTier _returnvalue_7)
          (CallFunction|CEDecal "PosY" _returnvalue_7))
        (else
          (bind _returnvalue_8 (AddComponent|AddStaticMeshComponent false (Math|Transform|MakeTransform (Math|Vector|MakeVector (.x (.location _returnvalue_2)) (+ (.y (.location _returnvalue_2)) _offset_2) (.z (.location _returnvalue_2))) (.rotation _returnvalue_2) (* (.scale _returnvalue_2) (Variables|Default|GetSide%20Size)))))
          (Components|StaticMesh|SetStaticMesh _returnvalue_8 (Utilities|Array|Get(acopy) _decals (Math|Random|RandomInteger (Utilities|Array|Length _decals))))
          (CallFunction|SpawnTier _returnvalue_8)
          (if (>= (Math|Random|RandomFloat) 0.1)
            (CallFunction|SideTier _returnvalue_8)
            (CallFunction|CEDecal "NegY" _returnvalue_8)))))))

(event Custom|CE_Decal
  (params (Direction :type String) (SM :type Static%20Mesh%20Component%20Object%20Reference))
  (bind _returnvalue (Transformation|GetRelativeTransform SM))
  (bind _returnvalue_2 (Transformation|GetRelativeTransform SM))
  (bind _returnvalue_3 (Transformation|GetRelativeTransform SM))
  (bind _returnvalue_4 (Transformation|GetRelativeTransform SM))
  (bind _offset (Variables|Default|GetOffset))
  (bind _decal_gap (Variables|Default|GetDecal%20Gap))
  (bind _decals (Variables|Default|GetDecals))
  (bind _decals_2 (Variables|Default|GetDecals))
  (bind _decals_3 (Variables|Default|GetDecals))
  (bind _decals_4 (Variables|Default|GetDecals))
  (bind (_x _y) (Math|Vector|BreakVector (.scale _returnvalue_3)))
  (bind (_x_2 _y_2) (Math|Vector|BreakVector (.scale _returnvalue)))
  (bind (_x_3 _y_3) (Math|Vector|BreakVector (.scale _returnvalue_4)))
  (bind (_x_4 _y_4) (Math|Vector|BreakVector (.scale _returnvalue_2)))
  (bind _returnvalue_5 (/ _offset 1e+03))
  (bind _returnvalue_6 (* _decal_gap _returnvalue_5))
  (if (>= (Math|Random|RandomFloat) 0.9)
    (switch string Direction
      (:PosX
        (bind _returnvalue_7 (AddComponent|AddStaticMeshComponent false (Math|Transform|MakeTransform (Math|Vector|MakeVector (+ (.x (.location _returnvalue)) _returnvalue_6) (.y (.location _returnvalue)) (.z (.location _returnvalue))) "90.000000,0.000000,0.000000" (Math|Vector|MakeVector _x_2 _y_2 0.1))))
        (Components|StaticMesh|SetStaticMesh _returnvalue_7 (Utilities|Array|Get(acopy) _decals (Math|Random|RandomInteger (Utilities|Array|Length _decals)))))
      (:NegX
        (bind _returnvalue_8 (AddComponent|AddStaticMeshComponent false (Math|Transform|MakeTransform (Math|Vector|MakeVector (- (.x (.location _returnvalue_3)) _returnvalue_6) (.y (.location _returnvalue_3)) (.z (.location _returnvalue_3))) "90.000000,0.000000,0.000000" (Math|Vector|MakeVector _x _y 0.1))))
        (Components|StaticMesh|SetStaticMesh _returnvalue_8 (Utilities|Array|Get(acopy) _decals_4 (Math|Random|RandomInteger (Utilities|Array|Length _decals_4)))))
      (:PosY
        (bind _returnvalue_9 (AddComponent|AddStaticMeshComponent false (Math|Transform|MakeTransform (Math|Vector|MakeVector (.x (.location _returnvalue_4)) (- (.y (.location _returnvalue_4)) _returnvalue_6) (.z (.location _returnvalue_4))) "90.000000,90.000000,0.000000" (Math|Vector|MakeVector _x_3 _y_3 0.1))))
        (Components|StaticMesh|SetStaticMesh _returnvalue_9 (Utilities|Array|Get(acopy) _decals_3 (Math|Random|RandomInteger (Utilities|Array|Length _decals_3)))))
      (:NegY
        (bind _returnvalue_10 (AddComponent|AddStaticMeshComponent false (Math|Transform|MakeTransform (Math|Vector|MakeVector (.x (.location _returnvalue_2)) (+ (.y (.location _returnvalue_2)) _returnvalue_6) (.z (.location _returnvalue_2))) "90.000000,90.000000,0.000000" (Math|Vector|MakeVector _x_4 _y_4 0.1))))
        (Components|StaticMesh|SetStaticMesh _returnvalue_10 (Utilities|Array|Get(acopy) _decals_2 (Math|Random|RandomInteger (Utilities|Array|Length _decals_2))))))))

(event Custom|CE_Activate
  (Utilities|FlowControl|Delay 0.01)
  (CallFunction|SpawnTier (Variables|Default|GetCube)))

(event Custom|BuildY
  (bind _returnvalue (Transformation|GetActorTransform))
  ;[0.15 0.05645 0 0.5] DEP
  (Variables|Default|SetBonusY (- (Variables|Default|GetBonusY) 1e+03))
  (Game|SpawnActorfromClass "BP_Generator_C" (Math|Transform|MakeTransform (Math|Vector|MakeVector (+ (.x (.location _returnvalue)) (Variables|Default|GetBonusX)) (+ (.y (.location _returnvalue)) (Variables|Default|GetBonusY)) (.z (.location _returnvalue))) (.rotation _returnvalue) (.scale _returnvalue)) "Undefined" "MultiplyWithRoot" 0 0 :!label _label)
  (if (>= (Variables|Default|GetBonusY) 0.0)
    (Variables|Default|SetBonusY (- (Variables|Default|GetBonusY) 1e+03))
    (Utilities|FlowControl|Delay 0.1)
    (goto _label)
    (elif (not (== (Variables|Default|GetBonusX) 0.0))
      (Variables|Default|SetBonusX 0.0)
      (Variables|Default|SetBonusY (+ (* (Variables|Default|GetScale) 1e+03) (Variables|Default|GetBonusY)))
      (Utilities|FlowControl|Delay 0.1)
      (goto _label))))

(event EventBeginPlay
  (Variables|Default|SetOffset (* (.X (Math|Vector|BreakVector (.scale (Transformation|GetActorTransform)))) -1e+02))
  (Utilities|FlowControl|Delay 0.01)
  (CallFunction|CEActivate))

(fn ConstructionScript)