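; BP_Player is a team-based actor that moves itself in timed steps, with its Plane material picked by Team at construction.
; On BeginPlay, team one steps along Y, while team two offsets X and Y using look-at rotation roll and pitch toward player zero, rather than a direction vector.
; Both loop on short delays.
; Hits and Box overlaps jump the actor along Y against its team's Direction.
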(event OnComponentBeginOverlap(Box)
  (params (OverlappedComponent :type Primitive%20Component%20Object%20Reference) (OtherActor :type Actor%20Object%20Reference) (OtherComp :type Primitive%20Component%20Object%20Reference) (OtherBodyIndex :type Integer) (bFromSweep :type Boolean) (SweepResult :type Hit%20Result%20Structure%20%28by%20ref%29))
  (bind _returnvalue (Transformation|GetActorLocation))
  (bind (_x _y _z) (Math|Vector|BreakVector _returnvalue))
  (Transformation|SetActorLocation (Math|Vector|MakeVector _x (+ _y (* (Variables|Default|GetDirection) -2e+02)) _z) false false))

(event EventBeginPlay
  (bind _returnvalue (Transformation|GetActorLocation))
  (bind _returnvalue_2 (Game|GetPlayerCharacter 0))
  (bind _self self)
  (bind (_x _y _z) (Math|Vector|BreakVector _returnvalue))
  (bind _returnvalue_3 (Transformation|GetActorLocation _returnvalue_2))
  (bind _returnvalue_4 (Transformation|GetActorLocation _self))
  (bind _returnvalue_5 (Math|Rotator|FindLookatRotation _returnvalue_4 _returnvalue_3))
  (bind (_x_2 _y_2 _z_2) (Math|Vector|BreakVector _returnvalue_4))
  (bind (_roll _pitch) (Math|Rotator|BreakRotator _returnvalue_5))
  (switch int (- (Variables|Default|GetTeam) 1)
    (:0
      (Variables|Default|SetDirection 1.0)
      (Transformation|SetActorLocation (Math|Vector|MakeVector _x (+ _y (* (Variables|Default|GetDirection) 1.5e+02)) _z) false false :!label _label)
      (Utilities|FlowControl|Delay 0.2)
      (goto _label))
    (:1
      (Variables|Default|SetDirection -2.0)
      (Transformation|SetActorLocation (Math|Vector|MakeVector (+ (* _roll -9e+01) _x_2) (+ (* _pitch -9e+01) _y_2) _z_2) false false :!label _label_2)
      (Utilities|FlowControl|Delay 0.2)
      (goto _label_2))))

(event Collision|EventHit
  (params (MyComp :type Primitive%20Component%20Object%20Reference) (Other :type Actor%20Object%20Reference) (OtherComp :type Primitive%20Component%20Object%20Reference) (bSelfMoved :type Boolean) (HitLocation :type Vector :default "0, 0, 0") (HitNormal :type Vector :default "0, 0, 0") (NormalImpulse :type Vector :default "0, 0, 0") (Hit :type Hit%20Result%20Structure%20%28by%20ref%29))
  (bind _returnvalue (Transformation|GetActorLocation))
  (bind (_x _y _z) (Math|Vector|BreakVector _returnvalue))
  (Transformation|SetActorLocation (Math|Vector|MakeVector _x (+ _y (* (Variables|Default|GetDirection) -2e+02)) _z) false false))

(fn ConstructionScript
  (Rendering|Material|SetMaterial (Variables|Default|GetPlane) 0 (Utilities|Array|Get(acopy) (Variables|Default|GetMaterial) (- (Variables|Default|GetTeam) 1))))