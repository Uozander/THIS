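; BP_Bouncy is a bouncing actor that kicks itself in a random direction and leaves a decal on whatever it hits.
; Each static mesh hit adds a random impulse on all three axes as a velocity change, so mass is ignored.
; The same hit spawns a BP_Decal actor at the impact point, rotated along the surface normal.
; An unconnected SpawnDecalAtLocation node remains in the graph and never runs.
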(event OnComponentHit(StaticMesh)
  (params (HitComponent :type Primitive%20Component%20Object%20Reference) (OtherActor :type Actor%20Object%20Reference) (OtherComp :type Primitive%20Component%20Object%20Reference) (NormalImpulse :type Vector :default "0, 0, 0") (Hit :type Hit%20Result%20Structure%20%28by%20ref%29))
  (Physics|AddImpulse (Variables|Default|GetStaticMesh) (Math|Vector|MakeVector (* (- (Math|Random|RandomFloat) 0.5) 3e+03) (* (- (Math|Random|RandomFloat) 0.5) 3e+03) (* (- (Math|Random|RandomFloat) 0.5) 3e+03)) "None" true)
  (Game|SpawnActorfromClass "/Game/BP_Decal.BP_Decal_C" (Math|Transform|MakeTransform (.impactpoint Hit) (Math|Conversions|RotationFromXVector (.normal Hit)) "1.000000,1.000000,1.000000") "Undefined" "MultiplyWithRoot" 0 0))

(fn ConstructionScript)